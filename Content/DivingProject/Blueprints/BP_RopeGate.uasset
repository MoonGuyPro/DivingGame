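; BP_RopeGate is an interactable gate actor that is removed when the player uses it while holding the required item kind.
; Overlapping UseSphere shows the Interact prompt and registers the gate as the first-person character's CurrentRopeGateNearby, clearing it on exit.
; TryUse checks Opened, then destroys the gate if the held item's kind matches RequiredKind.
; The WrongItem prompt appears only when no valid item is held; a mismatched item does nothing.
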(event OnComponentBeginOverlap(UseSphere)
  (params (OverlappedComponent :type Primitive%20Component%20Object%20Reference) (OtherActor :type Actor%20Object%20Reference) (OtherComp :type Primitive%20Component%20Object%20Reference) (OtherBodyIndex :type Integer) (bFromSweep :type Boolean) (SweepResult :type Hit%20Result%20Structure%20%28by%20ref%29))
  (bind _asbp_first_person_character (Utilities|Casting|CastToBP_FirstPersonCharacter OtherActor))
  (Rendering|SetVisibility (Variables|Default|GetInteract) true false)
  (Variables|/Game/FirstPerson/Blueprints/BP_FirstPersonCharacter.BP_FirstPersonCharacter_C|SetCurrentRopeGateNearby _asbp_first_person_character self))

(event OnComponentEndOverlap(UseSphere)
  (params (OverlappedComponent :type Primitive%20Component%20Object%20Reference) (OtherActor :type Actor%20Object%20Reference) (OtherComp :type Primitive%20Component%20Object%20Reference) (OtherBodyIndex :type Integer))
  (bind _asbp_first_person_character (Utilities|Casting|CastToBP_FirstPersonCharacter OtherActor))
  (Rendering|SetVisibility (Variables|Default|GetInteract) false false)
  (if (== (Variables|/Game/FirstPerson/Blueprints/BP_FirstPersonCharacter.BP_FirstPersonCharacter_C|GetCurrentRopeGateNearby _asbp_first_person_character) self)
    (Variables|/Game/FirstPerson/Blueprints/BP_FirstPersonCharacter.BP_FirstPersonCharacter_C|SetCurrentRopeGateNearby _asbp_first_person_character 0)
    (Rendering|SetVisibility (Variables|Default|GetWrongItem) false false)))

(event Custom|TryUse
  (params (PlayerRef :type BP%20First%20Person%20Character%20Object%20Reference))
  (bind _helditem (Variables|/Game/FirstPerson/Blueprints/BP_FirstPersonCharacter.BP_FirstPersonCharacter_C|GetHeldItem PlayerRef))
  (if (not (Variables|Default|GetbOpened))
    (if (Utilities|IsValid _helditem)
      (if (Utilities|Enum|Equal(Enum) (Variables|/Game/DivingProject/Blueprints/BP_PickupItem.BP_PickupItem_C|GetItemKind _helditem) (Variables|Default|GetRequiredKind))
        (Actor|DestroyActor))
      (else
        (Rendering|SetVisibility (Variables|Default|GetWrongItem) true false)))))

(event EventBeginPlay)

(event Collision|EventActorBeginOverlap
  (params (OtherActor :type Actor%20Object%20Reference)))

(event EventTick
  (params (DeltaSeconds :type Float%20%28single-precision%29)))

(fn ConstructionScript)