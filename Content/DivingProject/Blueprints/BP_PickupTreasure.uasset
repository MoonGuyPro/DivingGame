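; BP_PickupTreasure is a treasure pickup actor in the diving project that shows a world-space prompt when the player is near.
; Overlapping its PickupSphere as BP_FirstPersonCharacter reveals PromptWidget and stores the character in PlayerRef, while leaving hides the widget.
; Every tick the widget turns toward the player character using a look-at rotation from the actor's location.
; The graph contains no collection logic.
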(event OnComponentBeginOverlap(PickupSphere)
  (params (OverlappedComponent :type Primitive%20Component%20Object%20Reference) (OtherActor :type Actor%20Object%20Reference) (OtherComp :type Primitive%20Component%20Object%20Reference) (OtherBodyIndex :type Integer) (bFromSweep :type Boolean) (SweepResult :type Hit%20Result%20Structure%20%28by%20ref%29))
  (bind _asbp_first_person_character (Utilities|Casting|CastToBP_FirstPersonCharacter OtherActor))
  (Rendering|SetVisibility (Variables|Default|GetPromptWidget) true false)
  (Variables|Default|SetPlayerRef _asbp_first_person_character))

(event OnComponentEndOverlap(PickupSphere)
  (params (OverlappedComponent :type Primitive%20Component%20Object%20Reference) (OtherActor :type Actor%20Object%20Reference) (OtherComp :type Primitive%20Component%20Object%20Reference) (OtherBodyIndex :type Integer))
  (Utilities|Casting|CastToBP_FirstPersonCharacter OtherActor)
  (Rendering|SetVisibility (Variables|Default|GetPromptWidget) false false))

(event EventBeginPlay)

(event Collision|EventActorBeginOverlap
  (params (OtherActor :type Actor%20Object%20Reference)))

(event EventTick
  (params (DeltaSeconds :type Float%20%28single-precision%29))
  (Transformation|SetWorldRotation (Variables|Default|GetPromptWidget) (Math|Rotator|FindLookatRotation (Transformation|GetActorLocation) (Transformation|GetActorLocation (Game|GetPlayerCharacter 0))) false false))

(fn ConstructionScript)