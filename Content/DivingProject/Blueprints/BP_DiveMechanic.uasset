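; BP_DiveMechanic is a component that sets up state for a diving mechanic with helmet pressure and pump rate.
; StartDive activates the dive, records the owner's starting Y, stores target and descent speed, and resets pump, timer and helmet pressure.
; An unconnected chain derives depth from Y drop, then ambient pressure and a safe band around it, but never runs.
; BeginPlay and Tick are empty, so nothing updates during the dive.
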(event Custom|StartDive
  (params (TargetY :type Float%20%28double-precision%29) (DescentSpeedIn :type Float%20%28double-precision%29))
  (Variables|Default|SetDiveActive true)
  (Variables|Default|SetStartY (.Y (Math|Vector|BreakVector (Transformation|GetActorLocation (Components|GetOwner)))))
  (Variables|Default|SetTargetY TargetY)
  (Variables|Default|SetDescentSpeed DescentSpeedIn)
  (Variables|Default|SetPumpRateCurrent 0.0)
  (Variables|Default|SetBelowMinTimer 0.0)
  (Variables|Default|SetPressureHelmet (Variables|Default|GetAmbientAtSurface)))

(event EventBeginPlay)

(event EventTick
  (params (DeltaSeconds :type Float%20%28single-precision%29)))