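; BP_PickupItem is a world item that the first-person character can pick up and drop.
; Its sphere overlap toggles a prompt widget, turned toward the player every Tick, and sets or clears the character's CurrentItemNerby.
; OnPickedUp hides the actor, disables collision and becomes the player's HeldItem.
; OnDropped restores it at the player's location and clears that reference, but leaves IsHeld true.
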(event OnComponentBeginOverlap(PickupSphere)
  (params (OverlappedComponent :type Primitive%20Component%20Object%20Reference) (OtherActor :type Actor%20Object%20Reference) (OtherComp :type Primitive%20Component%20Object%20Reference) (OtherBodyIndex :type Integer) (bFromSweep :type Boolean) (SweepResult :type Hit%20Result%20Structure%20%28by%20ref%29))
  (bind _asbp_first_person_character (Utilities|Casting|CastToBP_FirstPersonCharacter OtherActor))
  (Rendering|SetVisibility (Variables|Default|GetPromptWidget) true false)
  (Variables|/Game/FirstPerson/Blueprints/BP_FirstPersonCharacter.BP_FirstPersonCharacter_C|SetCurrentItemNerby _asbp_first_person_character self))

(event OnComponentEndOverlap(PickupSphere)
  (params (OverlappedComponent :type Primitive%20Component%20Object%20Reference) (OtherActor :type Actor%20Object%20Reference) (OtherComp :type Primitive%20Component%20Object%20Reference) (OtherBodyIndex :type Integer))
  (bind _asbp_first_person_character (Utilities|Casting|CastToBP_FirstPersonCharacter OtherActor))
  (Rendering|SetVisibility (Variables|Default|GetPromptWidget) false false)
  (if (== (Variables|/Game/FirstPerson/Blueprints/BP_FirstPersonCharacter.BP_FirstPersonCharacter_C|GetCurrentItemNerby _asbp_first_person_character) self)
    (Variables|/Game/FirstPerson/Blueprints/BP_FirstPersonCharacter.BP_FirstPersonCharacter_C|SetCurrentItemNerby _asbp_first_person_character 0)))

(event Custom|OnPickedUp
  (params (PlayerRef :type BP%20First%20Person%20Character%20Object%20Reference))
  (Variables|Default|SetOwnerPlayer PlayerRef)
  (Variables|Default|SetbIsHeld true)
  (Rendering|SetActorHiddenInGame true)
  (Collision|SetActorEnableCollision false)
  (Variables|/Game/FirstPerson/Blueprints/BP_FirstPersonCharacter.BP_FirstPersonCharacter_C|SetHeldItem PlayerRef self))

(event Custom|OnDropped
  (params (PlayerRef :type BP%20First%20Person%20Character%20Object%20Reference))
  (Variables|Default|SetOwnerPlayer 0)
  (Variables|Default|SetbIsHeld true)
  (Rendering|SetActorHiddenInGame false)
  (Collision|SetActorEnableCollision true)
  (Transformation|SetActorLocation (Transformation|GetActorLocation PlayerRef) false false)
  (Variables|/Game/FirstPerson/Blueprints/BP_FirstPersonCharacter.BP_FirstPersonCharacter_C|SetHeldItem PlayerRef 0))

(event EventBeginPlay)

(event Collision|EventActorBeginOverlap
  (params (OtherActor :type Actor%20Object%20Reference)))

(event EventTick
  (params (DeltaSeconds :type Float%20%28single-precision%29))
  (Transformation|SetWorldRotation (Variables|Default|GetPromptWidget) (Math|Rotator|FindLookatRotation (Transformation|GetActorLocation) (Transformation|GetActorLocation (Game|GetPlayerCharacter 0))) false false))

(fn ConstructionScript)